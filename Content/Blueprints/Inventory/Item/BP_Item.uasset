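; BP_Item is an inventory item that loads its stats from a data table and can add them to the player's base stats.
; On BeginPlay it looks up its ID in DT_Items, copies stats, type and name, then writes name and quantity to its pickup label widget.
; The test onEquip event calls FuncUpdateStats, which adds values only where both stat maps share a key at the same index.
; The Unequipping input is unused, so stats are never subtracted.
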(event Custom|onEquip
  ;[1 1 1] Evt_onEquip: Apply stats (testing).
  (Equipping|FuncUpdateStats (.AsChar%20Player (Utilities|Casting|CastToChar_Player (Game|GetPlayerCharacter 0))) false))

(event EventBeginPlay
  ;[1 1 1] Evt_BeginPlay: Initialise the item stats.
  (Initialise|FuncInitialise))

(fn ConstructionScript)

(fn FuncInitialise
  ;[1 1 1] Retrieve stats from data table.
  (bind _returnvalue (Utilities|GetDataTableRow "/Game/Data/Tables/DT_Items.DT_Items" (Utilities|String|StringToName (Variables|Stats|Getstr_ItemID)))
    (:then
      (Utilities|FlowControl|Sequence
        (:then_0
          (Variables|Stats|SetfloM_Stats (.floM_Stats (Utilities|Struct|BreakDS_Items _returnvalue))))
        (:then_1
          (Variables|Stats|Setenum_ItemType (.enum_ItemType (Utilities|Struct|BreakDS_Items _returnvalue))))
        (:then_2
          (Variables|Stats|Setstr_ItemName (.str_ItemName (Utilities|Struct|BreakDS_Items _returnvalue))))
        (:then_3
          ;[1 1 1] Update item label (only for pickup).
          (Variables|/Game/Blueprints/UI/Gameplay/WID_ItemLabel.WID_ItemLabel_C|Settxt_ItemName (.AsWID%20Item%20Label (Utilities|Casting|CastToWID_ItemLabel (UserInterface|GetUserWidgetObject (Variables|Default|GetWBP_ItemLabel)))) (Utilities|Text|FormatText "{ItemName}    x{Quantity}" (Utilities|Text|ToText(String) (Variables|Stats|Getstr_ItemName)) (Variables|Stats|Getint_Quantity))))))))

(fn FuncUpdateStats
  (params (Player :type Char%20Player%20Object%20Reference) (Unequipping? :type Boolean))
  (bind _flom_basestats (Variables|/Game/Blueprints/Character/Char_Player.Char_Player_C|GetfloM_BaseStats Player))
  (bind _flom_stats (Variables|Stats|GetfloM_Stats))
  ;[1 1 1] Local variable setup for parsing map into two arrays.
  (LocalVariables|Setlact_PlayerReference Player)
  (Utilities|FlowControl|Sequence
    (:then_0
      (bind _values (Utilities|Map|Values _flom_basestats))
      (LocalVariables|SetlfloA_CharValues _values))
    (:then_1
      (bind _keys (Utilities|Map|Keys _flom_basestats))
      (LocalVariables|SetlenumA_CharKeys _keys))
    (:then_2
      (bind _values_2 (Utilities|Map|Values _flom_stats))
      (LocalVariables|SetlfloA_ItemValues _values_2))
    (:then_3
      (bind _keys_2 (Utilities|Map|Keys _flom_stats))
      (LocalVariables|SetlenumA_ItemKeys _keys_2))
    (:then_4
      ;[1 1 1] Loops through each of the player's stats and adds them with the item stats IF they are of the same stat type.
      (for (_array_element _array_index) (LocalVariables|GetlfloA_CharValues)
        (if (Utilities|Enum|Equal(Enum) (Utilities|Array|Get(acopy) (LocalVariables|GetlenumA_CharKeys) _array_index) (Utilities|Array|Get(acopy) (LocalVariables|GetlenumA_ItemKeys) _array_index))
          (Utilities|Map|Add (Variables|/Game/Blueprints/Character/Char_Player.Char_Player_C|GetfloM_BaseStats (LocalVariables|Getlact_PlayerReference)) (Utilities|Array|Get(acopy) (LocalVariables|GetlenumA_CharKeys) _array_index) (+ _array_element (Utilities|Array|Get(acopy) (LocalVariables|GetlfloA_ItemValues) _array_index))))))))